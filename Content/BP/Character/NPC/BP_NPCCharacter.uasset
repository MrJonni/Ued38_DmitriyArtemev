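; NPC character that takes damage into its main stats component and shows health through an HP bar widget and floating text.
; Any actor overlap applies fixed self-damage, which AnyDamage forwards to the component using the BP_DamageObject type.
; LookAtCamera turns the text toward the camera of the AI controller's targeted player.
; A stats-update handler refreshes the text and destroys the NPC on death, though its binding here is unconnected.
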(event `self.ReceiveBeginPlay`
  (`parent.ReceiveBeginPlay`)
  (bind _asw_health_bar (cast `/Game/BP/HUD/Widgets/W_HealthBar` (`WidgetComponent.GetUserWidgetObject` (`self.WidgetHP`))))
  (`/Game/BP/HUD/Widgets/W_HealthBar.UpdateCurrentCharacterForHP` _asw_health_bar self))

(event `self.ReceiveActorBeginOverlap`
  (params (OtherActor :type "Actor Object Reference"))
  (`parent.ReceiveActorBeginOverlap` OtherActor)
  (`GameplayStatics.ApplyDamage` self 50.0 null null "/Game/BP/Objects/BP_DamageObject.BP_DamageObject_C"))

(event `OnDeath`
  ;[1 1 1] Умирают но не исчезают(просто перестают быть активными)
  (`KismetSystemLibrary.Delay` 0.1)
  (`self.K2_DestroyActor`))

(fn `ActionMain`
  (params (IsPressed :type Boolean))
  (`parent.ActionMain` IsPressed)
  (if (`self.IsActionMainPressed`)
    (`KismetSystemLibrary.PrintString` "Bang" true false (struct :`R` 1.0 :`G` 0.089927 :`B` 0.169615 :`A` 1.0) 1.0)))

(fn `AnyDamage`
  (params (Damage :type "Float (double-precision)" :default 0.0) (DamageType :type "DamageType Object Reference") (InstigatedBy :type "Controller Object Reference") (DamageCauser :type "Actor Object Reference"))
  (bind _asbp_damage_object (cast `/Game/BP/Objects/BP_DamageObject` DamageType))
  (`/Game/BP/Components/BP_MainStatsComponent.ReceiveDamage` (`self.BP_MainStatsComponent`) (`self.Damage`) (`/Game/BP/Objects/BP_DamageObject.DamageType` _asbp_damage_object) (`self.DamageCauser`)))

(fn `LookAtCamera`
  (if (`self.LookAt`)
    (bind _asbp_ai_controller (cast `/Game/BP/Controllers/BP_AiController` (`self.GetController`)))
    (bind _targetcharacter (`/Game/BP/Controllers/BP_AiController.TargetCharacter` _asbp_ai_controller)
      (:`then`
        (bind _asbp_player_character (cast `/Game/BP/Character/Player/BP_PlayerCharacter` _targetcharacter))
        (set `self.CameraLocation` (`SceneComponent.K2_GetComponentLocation` (`/Game/BP/Character/Player/BP_PlayerCharacter.Camera` _asbp_player_character)))
        (`SceneComponent.K2_SetWorldRotation` (`self.Text`) (`KismetMathLibrary.FindLookAtRotation` (`SceneComponent.K2_GetComponentLocation` (`self.Text`)) (`self.CameraLocation`)) false false))
      (:`else`))))

(fn `OnStatsUpdete`
  (params (CurrentHP :type Integer) (CurrentEP :type Integer) (IsDead :type Boolean) (IsItDamage :type Boolean))
  (bind _bp_mainstatscomponent (`self.BP_MainStatsComponent`))
  (`TextRenderComponent.K2_SetText` (`self.Text`) (select `bool` (`self.IsDead`) :`false` (`|FormatText` "HP{hp}/{maxhp}" (`/Game/BP/Components/BP_MainStatsComponent.CurrentHP` _bp_mainstatscomponent) (`.MaxHP_9_A771449D4D0FB6AC94A77181E18FF634` (break `/Game/BP/Structures/STRUCT_MainStats` (`/Game/BP/Components/BP_MainStatsComponent.MainStatsStructure` _bp_mainstatscomponent)))) :`true` (`|FormatText` "{A} IS DEAD" (`KismetSystemLibrary.GetDisplayName` self))))
  (if (`self.IsDead`)
    (`self.OnDeath`)))

(fn `UserConstructionScript`
  (`parent.UserConstructionScript`))