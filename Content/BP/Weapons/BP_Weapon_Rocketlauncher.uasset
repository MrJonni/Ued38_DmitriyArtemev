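; Rocket launcher weapon Blueprint whose only logic of its own is stat setup; its event graph holds just disabled stubs.
; ConfigureWeaponStats_0 looks up the given weapon name in DT_WeaponStats, stores the row and initializes current rounds and damage.
; Damage is then scaled by the DamageMult of the owner's BP_MainStatsComponent, if present, and truncated.
; An invalid name or missing row only prints an error.
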(fn `ConfigureWeaponStats_0`
  (params (InWeaponName :type Name))
  (bind _returnvalue (`self.GetOwner`))
  (bind _returnvalue_2 (`self.GetComponentByClass` _returnvalue "/Game/BP/Components/BP_MainStatsComponent.BP_MainStatsComponent_C"))
  (set `self.WeaponName` InWeaponName)
  (if (!= (`self.WeaponName`) "None")
    (bind _returnvalue_3 (`|GetDataTableRow` "/Game/Data/DT_WeaponStats.DT_WeaponStats" (`self.WeaponName`))
      (:`then`
        (set `self.WeaponStats` _returnvalue_3)
        (set `self.RoundsCurrent` (`.RoundsMax_14_B57F376945DAB8ED366654B4F67D7181` (break `/Game/BP/Structures/STRUCT_WeaponStats` (`self.WeaponStats`))))
        (set `self.DamageCurrent` (`.Damage_23_61E616324BCD3F6B72F6C28E4ACAA11B` (break `/Game/BP/Structures/STRUCT_WeaponStats` (`self.WeaponStats`))))
        (`/Engine/EditorBlueprintResources/StandardMacros.IsValid` _returnvalue
          (:`Is Valid`
            (`/Engine/EditorBlueprintResources/StandardMacros.IsValid` _returnvalue_2
              (:`Is Valid`
                (set `self.DamageCurrent` (`KismetMathLibrary.FTrunc` (* (`self.DamageCurrent`) (`.DamageMult_10_9B4C10054C5A7CC5BB7CF2A3341114A4` (break `/Game/BP/Structures/STRUCT_MainStats` (`/Game/BP/Components/BP_MainStatsComponent.MainStatsStructure` _returnvalue_2)))))))))))
      (:`RowNotFound`
        (`KismetSystemLibrary.PrintString` "Configure Weapon Stats Failed: Current Name not found in DT" false)))
    (else
      (`KismetSystemLibrary.PrintString` "Configure Weapon Stats Failed: Current Name Is Invalid" false))))

(fn `UserConstructionScript`
  (`parent.UserConstructionScript`))