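; Shotgun weapon Blueprint that extends a parent weapon class and fires a spread of pellets per shot.
; SingleShot replaces the parent version, spawning BP_Projectile_Shotgun actors from the muzzle in an evenly spaced yaw fan set by MaxBulletInShot and ShotAngle, then calls ShotEffects.
; ShotEffects defers to the parent, while weapon configuration runs the parent setup and then calls SetSkeletalMesh on the inherited pistol prop with no mesh specified.
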(fn `ConfigureWeaponStats_0`
  (params (InWeaponName :type Name :default "None"))
  (`parent.ConfigureWeaponStats` InWeaponName)
  (`SkinnedMeshComponent.SetSkinnedAssetAndUpdate` (`self.SK_Prop_Pistol_01`) null true))

(fn `ShotEffects`
  (`parent.ShotEffects`))

(fn `SingleShot`
  (locals (L_Integer :type Integer))
  (`|ExecutionSequence`
    (:`then_0`
      (for _index (range (+ (`self.MaxBulletInShot`) 1))
        (set `local.L_Integer` _index)
        (`|SpawnActorFromClass` "/Game/BP/Weapons/Projectiles/BP_Projectile_Shotgun.BP_Projectile_Shotgun_C" (`KismetMathLibrary.MakeTransform` (.location (`SceneComponent.K2_GetComponentToWorld` (`self.MuzzleScene`))) (`KismetMathLibrary.MakeRotator` (.roll (.rotation (`SceneComponent.K2_GetComponentToWorld` (`self.MuzzleScene`)))) (.pitch (.rotation (`SceneComponent.K2_GetComponentToWorld` (`self.MuzzleScene`)))) (+ (.yaw (.rotation (`SceneComponent.K2_GetComponentToWorld` (`self.MuzzleScene`)))) (* (- (`local.L_Integer`) (/ (`self.MaxBulletInShot`) 2)) (`self.ShotAngle`)))) (.scale (`SceneComponent.K2_GetComponentToWorld` (`self.MuzzleScene`)))) "AdjustIfPossibleButAlwaysSpawn" "OverrideRootScale" self null)))
    (:`then_1`
      (`self.ShotEffects`))))

(fn `UserConstructionScript`
  (`parent.UserConstructionScript`))