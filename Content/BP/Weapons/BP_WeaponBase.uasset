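; Base weapon Blueprint that handles firing, ammo, reloading and show/hide on activation.
; Stats load by name from DT_WeaponStats, with damage scaled by the owner's BP_MainStatsComponent.
; While active, Tick polls fire input and prints ammo; shots spawn a type-selected projectile plus sound and muzzle FX.
; A timer-driven state enum gates shots and reloads, which draw on the owner's BP_BackpackComponent when present and broadcast status changes.
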(event `self.ReceiveTick`
  (params (DeltaSeconds :type "Float (single-precision)"))
  (if (`self.IsWeaponActive`)
    (`|ExecutionSequence`
      (:`then_0`
        (`self.Shooting`))
      (:`then_1`
        (`KismetSystemLibrary.PrintString` (`KismetStringLibrary.Concat_StrStr` (`KismetStringLibrary.Conv_IntToString` (`self.RoundsCurrent`)) "/" (`KismetStringLibrary.Conv_IntToString` (`.RoundsMax_14_B57F376945DAB8ED366654B4F67D7181` (break `/Game/BP/Structures/STRUCT_WeaponStats` (`self.WeaponStats`))))) true false (struct :`G` 0.66 :`B` 1.0 :`A` 1.0) 0.0)))))

(event `/Game/BP/BPI_CustomInterface.ShootProcess`
  (params (InProcess :type Boolean))
  (`self.ShootInputRecived` InProcess))

(fn `ActivateWeapon`
  (params (InActivation :type Boolean))
  (locals (L_Skel_Mesh :type "Array of SkeletalMeshComponent Object Reference") (L_Stst_Mesh :type "Array of StaticMeshComponent Object Reference"))
  (set `self.IsWeaponActive` (`local.InActivation`))
  (`|ExecutionSequence`
    (:`then_0`
      (bind _output_get (set `local.L_Skel_Mesh` (`self.K2_GetComponentsByClass` "/Script/Engine.SkeletalMeshComponent")))
      (if (`KismetArrayLibrary.Array_IsValidIndex` _output_get)
        (for _array_element (`local.L_Skel_Mesh`)
          (`SceneComponent.SetVisibility` _array_element (`self.IsWeaponActive`) true))))
    (:`then_1`
      (bind _output_get_2 (set `local.L_Stst_Mesh` (`self.K2_GetComponentsByClass` "/Script/Engine.StaticMeshComponent")))
      (if (`KismetArrayLibrary.Array_IsValidIndex` _output_get_2)
        (for _array_element_2 (`local.L_Stst_Mesh`)
          (`SceneComponent.SetVisibility` _array_element_2 (`self.IsWeaponActive`) true))))))

(fn `AfterShotDelayEnds`
  (set `self.WeaponState` "NewEnumerator0"))

(fn `ConfigureWeaponStats`
  (params (InWeaponName :type Name))
  (bind _returnvalue (`self.GetOwner`))
  (bind _returnvalue_2 (`self.GetComponentByClass` _returnvalue "/Game/BP/Components/BP_MainStatsComponent.BP_MainStatsComponent_C"))
  (set `self.WeaponName` InWeaponName)
  (if (!= (`self.WeaponName`) "None")
    (bind _returnvalue_3 (`|GetDataTableRow` "/Game/Data/DT_WeaponStats.DT_WeaponStats" (`self.WeaponName`))
      (:`then`
        (set `self.WeaponStats` _returnvalue_3)
        (set `self.RoundsCurrent` (`.RoundsMax_14_B57F376945DAB8ED366654B4F67D7181` (break `/Game/BP/Structures/STRUCT_WeaponStats` (`self.WeaponStats`))))
        (set `self.DamageCurrent` (`.Damage_23_61E616324BCD3F6B72F6C28E4ACAA11B` (break `/Game/BP/Structures/STRUCT_WeaponStats` (`self.WeaponStats`))))
        (`/Engine/EditorBlueprintResources/StandardMacros.IsValid` _returnvalue
          (:`Is Valid`
            (`/Engine/EditorBlueprintResources/StandardMacros.IsValid` _returnvalue_2
              (:`Is Valid`
                (set `self.DamageCurrent` (`KismetMathLibrary.FTrunc` (* (`self.DamageCurrent`) (`.DamageMult_10_9B4C10054C5A7CC5BB7CF2A3341114A4` (break `/Game/BP/Structures/STRUCT_MainStats` (`/Game/BP/Components/BP_MainStatsComponent.MainStatsStructure` _returnvalue_2)))))))))))
      (:`RowNotFound`
        (`KismetSystemLibrary.PrintString` "Configure Weapon Stats Failed: Current Name not found in DT" false)))
    (else
      (`KismetSystemLibrary.PrintString` "Configure Weapon Stats Failed: Current Name Is Invalid" false))))

(fn `Interact`
  (returns (Success :type Boolean))
  (return false))

(fn `OnReloadDelayEnds`
  (set `self.WeaponState` "NewEnumerator0"))

(fn `Reaload`
  (bind _returnvalue (`self.GetComponentByClass` (`self.GetOwner`) "/Game/BP/Components/BP_BackpackComponent.BP_BackpackComponent_C"))
  (if (not (`self.In Process`))
    (set `self.WeaponState` "NewEnumerator3")
    (`AudioComponent.Play` (`self.ReloadStartSound`) 0.0)
    (`|ExecutionSequence`
      (:`then_0`
        (`/Engine/EditorBlueprintResources/StandardMacros.IsValid` _returnvalue
          (:`Is Valid`
            (bind _outammo (`/Game/BP/Components/BP_BackpackComponent.UpdateAmmoByName` _returnvalue (- (`.RoundsMax_14_B57F376945DAB8ED366654B4F67D7181` (break `/Game/BP/Structures/STRUCT_WeaponStats` (`self.WeaponStats`))) (`self.RoundsCurrent`)) false (`self.WeaponName`)))
            (set `self.RoundsCurrent` _outammo))
          (:`Is Not Valid`
            (set `self.RoundsCurrent` (`.RoundsMax_14_B57F376945DAB8ED366654B4F67D7181` (break `/Game/BP/Structures/STRUCT_WeaponStats` (`self.WeaponStats`)))))))
      (:`then_1`
        (if (!= (`self.RoundsCurrent`) 0)
          (`KismetSystemLibrary.K2_SetTimerDelegate` (`|CreateDelegate` :!event `OnReloadDelayEnds`) (`.ReloadTime_26_B497867441CBD76E114D109720877355` (break `/Game/BP/Structures/STRUCT_WeaponStats` (`self.WeaponStats`))))
          (`self.OnWeaponStatusChanged`)
          (else
            (set `self.WeaponState` "NewEnumerator4")
            (`self.OnWeaponStatusChanged`)))))))

(fn `RoundsCount`
  (returns (AllowShooting :type Boolean))
  (bind _result (`/Engine/EditorBlueprintResources/StandardMacros.DecrementInt` (`self.RoundsCurrent`))
    (:`  `
      (return (> _result 0)))))

(fn `Shooting`
  (if (and (`self.In Process`) (`|EnumEquality` (`self.WeaponState`) "NewEnumerator0"))
    (`self.SingleShot`)
    (bind _allowshooting (`self.RoundsCount`))
    (if _allowshooting
      (`KismetSystemLibrary.K2_SetTimerDelegate` (`|CreateDelegate` :!event `AfterShotDelayEnds`) (`.ShotTime_22_FF23810242B34E39376663B7FBE9A389` (break `/Game/BP/Structures/STRUCT_WeaponStats` (`self.WeaponStats`))))
      (set `self.WeaponState` "NewEnumerator1")
      (`self.OnWeaponStatusChanged`)
      (else
        (set `self.WeaponState` "NewEnumerator2")
        (if (`.AutoReload_29_8AF7AB5B4DD98AEC01C3118A7051B5B1` (break `/Game/BP/Structures/STRUCT_WeaponStats` (`self.WeaponStats`)))
          (`self.Reaload`)
          (else
            (`self.OnWeaponStatusChanged`)))))))

(fn `ShootInputRecived`
  (params (InProcess :type Boolean))
  (set `self.In Process` InProcess))

(fn `ShotEffects`
  (`AudioComponent.Play` (`self.ShootSound`) 0.0)
  (bind _returnvalue (`|SpawnActorFromClass` "/Game/BP/Weapons/Projectiles/BP_MuzzleFX.BP_MuzzleFX_C" (`SceneComponent.K2_GetComponentToWorld` (`self.MuzzleScene`)) "Undefined" "OverrideRootScale" null null))
  (`self.K2_AttachToComponent` _returnvalue (`self.MuzzleScene`) "None" "SnapToTarget" "SnapToTarget" "KeepRelative" true))

(fn `SingleShot`
  (bind _returnvalue (`|SpawnActorFromClass` (select `/Game/BP/Enum/ENUM_WeaponType` (`.WeaponType_3_6A77DB564F671686C3070CB3D2A3C1C9` (break `/Game/BP/Structures/STRUCT_WeaponStats` (`self.WeaponStats`))) :`NewEnumerator0` "/Game/BP/Weapons/Projectiles/BP_Projectile_Pistol.BP_Projectile_Pistol_C" :`NewEnumerator1` "/Game/BP/Weapons/Projectiles/BP_Projectile_Rifle.BP_Projectile_Rifle_C" :`NewEnumerator3` "/Game/BP/Weapons/Projectiles/BP_Projectile_Rocket.BP_Projectile_Rocket_C" :!type "Actor Class Reference") (`SceneComponent.K2_GetComponentToWorld` (`self.MuzzleArrow`)) "Undefined" "OverrideRootScale" self null))
  (cast `/Game/BP/Weapons/Projectiles/BP_ProjectileBase` _returnvalue)
  (`self.ShotEffects`))

(fn `UserConstructionScript`)