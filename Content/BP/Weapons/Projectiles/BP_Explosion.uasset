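; BP_Explosion is a projectile explosion actor that deals damage and physics impulses within its sphere radius on BeginPlay.
; SphereTraceCheck finds one object per trace, adds it to an ignore list and recurses until none remain, with debug drawing enabled.
; Each hit gets an outward, distance-scaled impulse if simulating physics, plus BP_DamageObject damage credited three owners up.
; A looping timer appears to drive RedyToDestroy, which destroys the actor once audio stops.
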(event `self.ReceiveBeginPlay`
  (`|ExecutionSequence`
    (:`then_0`
      (`self.SphereTraceCheck`))
    (:`then_1`
      (bind _returnvalue (`KismetSystemLibrary.K2_SetTimerDelegate` (`|CreateDelegate` :!event `RedyToDestroy`) 2.0 true))
      (set `self.Destroy` _returnvalue))))

(fn `AddPhisycsImpuls`
  (locals (NewLocalVar_0 :type "Float (double-precision)" :default 0.0))
  (bind _returnvalue (- (`self.K2_GetActorLocation` (`self.OtherActor`)) (`self.K2_GetActorLocation`)))
  (bind _otherhit_component (`self.OtherHit Component`)
    (:`then`
      (if (`SceneComponent.IsSimulatingPhysics` _otherhit_component "None")
        (`PrimitiveComponent.AddImpulseAtLocation` (`self.OtherHit Component`) (* _returnvalue (`KismetMathLibrary.Abs` (* (`KismetMathLibrary.MapRangeClamped` (`KismetMathLibrary.VSize` _returnvalue) 0.0 (`SphereComponent.SphereRadius` (`self.Sphere`)) 1.0 0.5) (`self.ImpulsMult`)))) (`self.K2_GetActorLocation`) "None")))
    (:`else`)))

(fn `MakeDamage`
  (`self.OtherActor`
    (:`then`
      (`GameplayStatics.ApplyDamage` (`self.OtherActor`) (`KismetMathLibrary.Conv_IntToDouble` (`self.ExplDamage`)) null (`self.GetOwner` (`self.GetOwner` (`self.GetOwner`))) "/Game/BP/Objects/BP_DamageObject.BP_DamageObject_C"))
    (:`else`)))

(fn `RedyToDestroy`
  (if (not (`AudioComponent.IsPlaying` (`self.Audio`)))
    (if (`KismetSystemLibrary.K2_IsValidTimerHandle` (`self.Destroy`))
      (`KismetSystemLibrary.K2_ClearAndInvalidateTimerHandle` (`self.Destroy`))
      (`self.K2_DestroyActor`))))

(fn `SphereTraceCheck`
  (bind _returnvalue (`self.K2_GetActorLocation` self))
  (bind (_outhit _returnvalue_2) (`KismetSystemLibrary.SphereTraceSingleForObjects` _returnvalue (+ _returnvalue (0.0 0.0 1.0)) (`SphereComponent.SphereRadius` (`self.Sphere`)) (`|MakeArray` "ObjectTypeQuery2" "ObjectTypeQuery3" "ObjectTypeQuery4" :!type "EObjectTypeQuery Enum") false (`self.InExplosionActor`) "ForDuration"))
  (if _returnvalue_2
    (bind (_bblockinghit _binitialoverlap _time _distance _location _impactpoint _normal _impactnormal _physmat _hitactor _hitcomponent) (`GameplayStatics.BreakHitResult` _outhit))
    (bind _output_get (set `self.OtherActor` _hitactor))
    (`KismetArrayLibrary.Array_AddUnique` (`self.InExplosionActor`) _output_get)
    (set `self.OtherHit Component` _hitcomponent)
    (`|ExecutionSequence`
      (:`then_0`
        (`self.AddPhisycsImpuls`))
      (:`then_1`
        (`self.MakeDamage`))
      (:`then_2`
        (`self.SphereTraceCheck`)))))

(fn `UserConstructionScript`)