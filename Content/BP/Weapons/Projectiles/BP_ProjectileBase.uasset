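; BP_ProjectileBase is the base weapon projectile, handling damage and impact effects when it hits something.
; On Hit it reads DamageCurrent from its owning BP_WeaponBase, triples it for "head" bone hits, and applies it with the weapon's owner as damage causer.
; It then spawns a randomly rolled impact effect aligned to the surface normal, attaches it to the hit component's bone, and destroys itself.
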(event `self.ReceiveHit`
  (params (MyComp :type "PrimitiveComponent Object Reference") (Other :type "Actor Object Reference") (OtherComp :type "PrimitiveComponent Object Reference") (bSelfMoved :type Boolean) (HitLocation :type "Vector Structure") (HitNormal :type "Vector Structure") (NormalImpulse :type "Vector Structure") (Hit :type "HitResult Structure (by ref)"))
  (set `self.Other` Other)
  (set `self.OtherComp` OtherComp)
  (set `self.Hit Location` HitLocation)
  (set `self.Hit Normal` HitNormal)
  (set `self.HitResult` Hit)
  (`|ExecutionSequence`
    (:`then_0`
      (`self.ApplyDamageByProjectile`))
    (:`then_1`
      (`self.SpawnDecal`))
    (:`then_2`
      (`self.OnEndOfHit`))))

(fn `ApplyDamageByProjectile`
  (locals (L_Damage :type Integer :default 0))
  (`|ExecutionSequence`
    (:`then_0`
      (bind _asbp_weapon_base (cast `/Game/BP/Weapons/BP_WeaponBase` (`self.GetOwner`)))
      (set `local.L_Damage` (`/Game/BP/Weapons/BP_WeaponBase.DamageCurrent` _asbp_weapon_base)))
    (:`then_1`
      (if (== (`.HitBoneName` (`GameplayStatics.BreakHitResult` (`self.HitResult`))) "head")
        (set `local.L_Damage` (* (`local.L_Damage`) 3))))
    (:`then_2`
      (`GameplayStatics.ApplyDamage` (`self.Other`) (`KismetMathLibrary.Conv_IntToDouble` (`local.L_Damage`)) null (`self.GetOwner` (`self.GetOwner`)) "/Game/BP/Objects/BP_DamageObject.BP_DamageObject_C"))))

(fn `OnEndOfHit`
  (`self.K2_DestroyActor`))

(fn `SpawnDecal`
  (locals (L_Rotation :type "Rotator Structure" :default (struct)) (L_Impact :type "/Game/BP/Weapons/Projectiles/BP_ImpactEffect Object Reference"))
  (bind (_returnvalue_roll _returnvalue_pitch _returnvalue_yaw) (`KismetMathLibrary.BreakRotator` (`KismetMathLibrary.Conv_VectorToRotator` (`self.Hit Normal`))))
  (set `local.L_Rotation` (`KismetMathLibrary.MakeRotator` (`KismetMathLibrary.RandomFloatInRange` 0.0 360.0) _returnvalue_pitch _returnvalue_yaw))
  (bind _returnvalue (`|SpawnActorFromClass` "/Game/BP/Weapons/Projectiles/BP_ImpactEffect.BP_ImpactEffect_C" (`KismetMathLibrary.MakeTransform` (`self.Hit Location`) (`local.L_Rotation`)) "Undefined" "OverrideRootScale" self null))
  (set `local.L_Impact` _returnvalue)
  (`self.K2_AttachToComponent` (`local.L_Impact`) (`self.OtherComp`) (`.HitBoneName` (`GameplayStatics.BreakHitResult` (`self.HitResult`))) "KeepWorld" "KeepWorld" "KeepWorld" true))

(fn `UserConstructionScript`)