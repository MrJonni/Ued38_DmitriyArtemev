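; Sniper rifle weapon Blueprint that overrides its parent's single shot with a hitscan line trace from the muzzle.
; On a hit it applies damage, tripled for the head bone, and spawns a randomly rolled impact effect attached to the struck component and bone.
; Every shot, hit or miss, plays the shoot sound and attaches a spawned muzzle effect.
; The trace ignores the rifle and its owner and leaves timed debug lines visible.
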(fn `ApplyDamageByProjectile`
  (locals (L_Damage :type Integer :default 0))
  (`|ExecutionSequence`
    (:`then_0`
      (set `local.L_Damage` (`self.DamageCurrent`)))
    (:`then_1`
      (if (== (`.HitBoneName` (`GameplayStatics.BreakHitResult` (`self.HitResult`))) "head")
        (set `local.L_Damage` (* (`local.L_Damage`) 3))))
    (:`then_2`
      (`GameplayStatics.ApplyDamage` (`self.Hit Actor`) (`KismetMathLibrary.Conv_IntToDouble` (`local.L_Damage`)) null (`self.GetOwner`) "/Game/BP/Objects/BP_DamageObject.BP_DamageObject_C"))))

(fn `ConfigureWeaponStats`
  (params (InWeaponName :type Name))
  (`parent.ConfigureWeaponStats` InWeaponName)
  (`SkinnedMeshComponent.SetSkinnedAssetAndUpdate` (`self.SK_Prop_Pistol_01`) null true))

(fn `ShotEffect`
  (`AudioComponent.Play` (`self.ShootSound`) 0.0)
  (bind _returnvalue (`|SpawnActorFromClass` "/Game/BP/Weapons/Projectiles/BP_MuzzleFX.BP_MuzzleFX_C" (`SceneComponent.K2_GetComponentToWorld` (`self.MuzzleScene`)) "Undefined" "OverrideRootScale" null null))
  (`self.K2_AttachToComponent` _returnvalue (`self.MuzzleScene`) "None" "SnapToTarget" "SnapToTarget" "KeepRelative" true))

(fn `SingleShot`
  (bind (_bblockinghit _binitialoverlap _time _distance _location _impactpoint _normal _impactnormal _physmat _hitactor _hitcomponent) (`GameplayStatics.BreakHitResult` (`self.HitResult`)))
  (bind _returnvalue (`SceneComponent.K2_GetComponentLocation` (`self.MuzzleScene`)))
  (`|ExecutionSequence`
    (:`then_0`
      (bind (_outhit _returnvalue_2) (`KismetSystemLibrary.LineTraceSingle` _returnvalue (+ _returnvalue (* (`SceneComponent.GetForwardVector` (`self.MuzzleScene`)) 10000.0)) "TraceTypeQuery2" true (`|MakeArray` self (`self.GetOwner`) :!type "Actor Object Reference") "ForDuration" true (struct :`R` 1.0 :`A` 1.0) (struct :`G` 1.0 :`A` 1.0) 10.0))
      (if _returnvalue_2
        (set `self.HitResult` _outhit)
        (set `self.Location` _location)
        (set `self.Normal` _normal)
        (set `self.Hit Actor` _hitactor)
        (set `self.Hit Component` _hitcomponent)
        (`|ExecutionSequence`
          (:`then_0`
            (`self.ApplyDamageByProjectile`))
          (:`then_1`
            (`self.SpawnDecal`)))))
    (:`then_1`
      (`self.ShotEffect`))))

(fn `SpawnDecal`
  (locals (L_Rotation :type "Rotator Structure" :default (struct)) (L_Impact :type "/Game/BP/Weapons/Projectiles/BP_ImpactEffect Object Reference"))
  (bind (_returnvalue_roll _returnvalue_pitch _returnvalue_yaw) (`KismetMathLibrary.BreakRotator` (`KismetMathLibrary.Conv_VectorToRotator` (`self.Normal`))))
  (set `local.L_Rotation` (`KismetMathLibrary.MakeRotator` (`KismetMathLibrary.RandomFloatInRange` 0.0 360.0) _returnvalue_pitch _returnvalue_yaw))
  (bind _returnvalue (`|SpawnActorFromClass` "/Game/BP/Weapons/Projectiles/BP_ImpactEffect.BP_ImpactEffect_C" (`KismetMathLibrary.MakeTransform` (`self.Location`) (`local.L_Rotation`)) "Undefined" "OverrideRootScale" self null))
  (set `local.L_Impact` _returnvalue)
  (`self.K2_AttachToComponent` (`local.L_Impact`) (`self.Hit Component`) (`.HitBoneName` (`GameplayStatics.BreakHitResult` (`self.HitResult`))) "KeepWorld" "KeepWorld" "KeepWorld" true))

(fn `UserConstructionScript`
  (`parent.UserConstructionScript`))