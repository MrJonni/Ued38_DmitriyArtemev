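; Tooltip actor whose text turns to face the player's camera while the player is inside its overlap area.
; Begin overlap sets a LookAt flag if CharacterInBox, which is not assigned in this Blueprint, is valid; any end overlap clears it.
; While the flag is set, Tick rotates the Text component toward the BP_PlayerCharacter camera using a look-at rotation.
; A LookAtCamera function duplicates the Tick logic but is not called here.
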(event `self.ReceiveTick`
  (params (DeltaSeconds :type "Float (single-precision)"))
  (`parent.ReceiveTick` DeltaSeconds)
  (if (`self.LookAt`)
    (bind _characterinbox (`self.CharacterInBox`)
      (:`then`
        (bind _asbp_player_character (cast `/Game/BP/Character/Player/BP_PlayerCharacter` _characterinbox))
        (set `self.CameraLocation` (`SceneComponent.K2_GetComponentLocation` (`/Game/BP/Character/Player/BP_PlayerCharacter.Camera` _asbp_player_character)))
        (`SceneComponent.K2_SetWorldRotation` (`self.Text`) (`KismetMathLibrary.FindLookAtRotation` (`SceneComponent.K2_GetComponentLocation` (`self.Text`)) (`self.CameraLocation`)) false false))
      (:`else`))))

(event `self.ReceiveActorBeginOverlap`
  (params (OtherActor :type "Actor Object Reference"))
  (`parent.ReceiveActorBeginOverlap` OtherActor)
  (`self.CharacterInBox`
    (:`then`
      (set `self.LookAt` true))
    (:`else`)))

(event `self.ReceiveActorEndOverlap`
  (params (OtherActor :type "Actor Object Reference"))
  (`parent.ReceiveActorEndOverlap` OtherActor)
  (set `self.LookAt` false))

(fn `LookAtCamera`
  (if (`self.LookAt`)
    (bind _characterinbox (`self.CharacterInBox`)
      (:`then`
        (bind _asbp_player_character (cast `/Game/BP/Character/Player/BP_PlayerCharacter` _characterinbox))
        (set `self.CameraLocation` (`SceneComponent.K2_GetComponentLocation` (`/Game/BP/Character/Player/BP_PlayerCharacter.Camera` _asbp_player_character)))
        (`SceneComponent.K2_SetWorldRotation` (`self.Text`) (`KismetMathLibrary.FindLookAtRotation` (`SceneComponent.K2_GetComponentLocation` (`self.Text`)) (`self.CameraLocation`)) false false))
      (:`else`))))

(fn `UserConstructionScript`
  (`parent.UserConstructionScript`))