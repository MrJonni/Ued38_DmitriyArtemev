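; BP_Tooltip is an environment tooltip actor that shows its Text component while the player character stands inside its box.
; Overlap events cast to BP_PlayerCharacter, store or clear CharacterInBox, and toggle the text's hidden-in-game state.
; The construction script sizes the box from BoxExtent, raises it by its half-height so its base sits at the parent's origin, and positions the text at TTL.
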(event `self.ReceiveActorBeginOverlap`
  (params (OtherActor :type "Actor Object Reference"))
  (bind _asbp_player_character (cast `/Game/BP/Character/Player/BP_PlayerCharacter` OtherActor))
  (set `self.CharacterInBox` _asbp_player_character)
  (`SceneComponent.SetHiddenInGame` (`self.Text`) false false))

(event `self.ReceiveActorEndOverlap`
  (params (OtherActor :type "Actor Object Reference"))
  (cast `/Game/BP/Character/Player/BP_PlayerCharacter` OtherActor)
  (set `self.CharacterInBox` null)
  (`SceneComponent.SetHiddenInGame` (`self.Text`) true false))

(fn `UserConstructionScript`
  (`BoxComponent.SetBoxExtent` (`self.BoxCollision`) (`self.Box Extent`) true)
  (`SceneComponent.K2_SetRelativeLocation` (`self.BoxCollision`) (`KismetMathLibrary.MakeVector` 0.0 0.0 (.z (`self.Box Extent`))) false false)
  (`SceneComponent.K2_SetRelativeLocation` (`self.Text`) (`self.TTL`) false false))