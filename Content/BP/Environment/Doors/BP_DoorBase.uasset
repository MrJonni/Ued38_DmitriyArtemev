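; Base door Blueprint that a character can open and close by interacting while standing near it.
; A Box overlap with BP_CharacterBase shows the Scene component hierarchy, hidden at start, and enables Interact, which toggles between opening and closing.
; One timeline, played forward or in reverse, scales the OpenDor yaw on DoorRotator, ignoring requests mid-swing and setting IsOpen when finished.
; The construction script pre-rotates doors that start open.
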(event `self.ReceiveBeginPlay`
  (`SceneComponent.SetVisibility` (`self.Scene`) false true))

(event `self.Box.OnComponentBeginOverlap`
  (params (OverlappedComponent :type "PrimitiveComponent Object Reference") (OtherActor :type "Actor Object Reference") (OtherComp :type "PrimitiveComponent Object Reference") (OtherBodyIndex :type Integer) (bFromSweep :type Boolean) (SweepResult :type "HitResult Structure (by ref)"))
  (bind _output_get (set `self.OverlappedActor` OtherActor))
  (cast `/Game/BP/Character/BP_CharacterBase` _output_get)
  (`SceneComponent.SetVisibility` (`self.Scene`) true true)
  (set `self.IsRedyToInteract` true))

(event `self.Box.OnComponentEndOverlap`
  (params (OverlappedComponent :type "PrimitiveComponent Object Reference") (OtherActor :type "Actor Object Reference") (OtherComp :type "PrimitiveComponent Object Reference") (OtherBodyIndex :type Integer))
  (set `self.OverlappedActor` null)
  (cast `/Game/BP/Character/BP_CharacterBase` OtherActor)
  (`SceneComponent.SetVisibility` (`self.Scene`) false true)
  (set `self.IsRedyToInteract` false))

(event `OpenDoor`
  (if (not (`self.InProgress`))
    (if (not (`self.IsOpen`))
      (bind (_direction _newtrack_0) (`Timeline|Timeline_0` :!via `PlayFromStart` :!label _label)
        (:`Update`
          (set `self.InProgress` true)
          (`SceneComponent.K2_SetRelativeRotation` (`self.DoorRotator`) (`KismetMathLibrary.MakeRotator` 0.0 0.0 (* (`self.OpenDor`) _newtrack_0)) false false))
        (:`Finished`
          (set `self.InProgress` false)
          (switch `ETimelineDirection` _direction
            (:`Forward`
              (set `self.IsOpen` true))
            (:`Backward`
              (set `self.IsOpen` false))))))))

(event `CloseDoor`
  (if (not (`self.InProgress`))
    (if (`self.IsOpen`)
      (goto _label :!via `ReverseFromEnd`))))

(fn `Interact`
  (returns (Success :type Boolean))
  (if (`self.IsRedyToInteract`)
    (if (`self.IsOpen`)
      (`self.CloseDoor`)
      (return true)
      (else
        (`self.OpenDoor`)
        (return true)))
    (else
      (return false))))

(fn `UserConstructionScript`
  (`SceneComponent.K2_AddRelativeRotation` (`self.DoorRotator`) (`KismetMathLibrary.MakeRotator` 0.0 0.0 (`KismetMathLibrary.SelectFloat` (`self.OpenDor`) 0.0 (`self.IsOpen`))) false false))