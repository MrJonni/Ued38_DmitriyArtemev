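; Lockable door Blueprint that extends a parent door, blocking opening while locked and showing lock state through a red or green indicator light.
; Interact toggles an unlocked door, or checks the overlapping actor's backpack component for the required key quest items.
; Found keys are removed even if the set is incomplete, and the door unlocks only when all match.
; Lock only takes effect on doors without required keys, while SwitchLock toggles freely.
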(event `self.OpenDoor`
  (if (not (`self.IsDoorLocked`))
    (`parent.OpenDoor`)))

(event `self.CloseDoor`
  (`parent.CloseDoor`))

(fn `DoorLockIndicator`
  (`LightComponent.SetLightColor` (`self.Lockindicator`) (`KismetMathLibrary.SelectColor` (struct :`R` 1.0 :`B` 0.04459 :`A` 1.0) (struct :`R` 0.083404 :`G` 0.427083 :`B` 0.076644 :`A` 1.0) (`self.IsDoorLocked`)) true))

(fn `Interact`
  (returns (Success :type Boolean))
  (locals (L_BackPack :type "/Game/BP/Components/BP_BackpackComponent Object Reference") (L_ItemInrement :type Integer) (L_ItemName :type Name))
  (if (`self.IsRedyToInteract`)
    (if (not (`self.IsDoorLocked`))
      (if (`self.IsOpen`)
        (`self.CloseDoor`)
        (return true)
        (else
          (`self.OpenDoor`)
          (return true)))
      (elif (`KismetArrayLibrary.Array_IsValidIndex` (`self.NeededKeyName`))
        (bind _overlappedactor (`self.OverlappedActor`)
          (:`then`
            (bind _returnvalue (`self.GetComponentByClass` _overlappedactor "/Game/BP/Components/BP_BackpackComponent.BP_BackpackComponent_C"))
            (`/Engine/EditorBlueprintResources/StandardMacros.IsValid` _returnvalue
              (:`Is Valid`
                (set `local.L_BackPack` _returnvalue)
                (for _array_element (`self.NeededKeyName`)
                  (set `local.L_ItemName` _array_element)
                  (if (`BlueprintSetLibrary.Set_Contains` (`/Game/BP/Components/BP_BackpackComponent.QuestItems` (`local.L_BackPack`)) (`local.L_ItemName`))
                    (`/Engine/EditorBlueprintResources/StandardMacros.IncrementInt` (`local.L_ItemInrement`)
                      (:`  `
                        (`/Game/BP/Components/BP_BackpackComponent.RemoveQuestItem` (`local.L_BackPack`) (`local.L_ItemName`))))))
                (if (== (`local.L_ItemInrement`) (`KismetArrayLibrary.Array_Length` (`self.NeededKeyName`)))
                  (`self.Unlock`)
                  (else
                    (return true))))
              (:`Is Not Valid`
                (return true))))
          (:`else`
            (return true)))
        (else
          (return true))))
    (else
      (return false))))

(fn `Lock`
  (if (not (`KismetArrayLibrary.Array_IsValidIndex` (`self.NeededKeyName`)))
    (set `self.IsDoorLocked` true)
    (`self.DoorLockIndicator`)))

(fn `SwitchLock`
  (set `self.IsDoorLocked` (not (`self.IsDoorLocked`)))
  (`self.DoorLockIndicator`))

(fn `Unlock`
  (set `self.IsDoorLocked` false)
  (`self.DoorLockIndicator`))

(fn `UserConstructionScript`
  (`parent.UserConstructionScript`)
  (`self.DoorLockIndicator`))