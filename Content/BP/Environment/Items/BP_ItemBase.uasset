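; BP_ItemBase is a base item actor that characters can interact with to put it into their backpack.
; Overlapping characters toggle a text prompt, which turns toward the BP_PlayerCharacter camera each tick, and a readiness flag.
; Interact passes the character's BP_BackpackComponent to PutIntoBackpack, an empty hook here, and returns true in every case.
; AfterUse destroys the actor.
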(event `self.ReceiveBeginPlay`
  (`SceneComponent.SetVisibility` (`self.Text`) false false))

(event `self.ReceiveActorBeginOverlap`
  (params (OtherActor :type "Actor Object Reference"))
  (bind _ascharacter (cast `Character` OtherActor))
  (set `self.CharacterInBox` _ascharacter)
  (`SceneComponent.SetVisibility` (`self.Text`) true false)
  (set `self.IsRedyToInteract` true)
  (set `self.LookAt` true))

(event `self.ReceiveActorEndOverlap`
  (params (OtherActor :type "Actor Object Reference"))
  (cast `Character` OtherActor)
  (set `self.CharacterInBox` null)
  (`SceneComponent.SetVisibility` (`self.Text`) false false)
  (set `self.IsRedyToInteract` false)
  (set `self.LookAt` false))

(event `self.ReceiveTick`
  (params (DeltaSeconds :type "Float (single-precision)"))
  (`self.LookAtCamera`))

(fn `AfterUse`
  (`self.K2_DestroyActor`))

(fn `Interact`
  (returns (Success :type Boolean))
  (if (`self.IsRedyToInteract`)
    (bind _characterinbox (`self.CharacterInBox`)
      (:`then`
        (bind _returnvalue (`self.GetComponentByClass` _characterinbox "/Game/BP/Components/BP_BackpackComponent.BP_BackpackComponent_C"))
        (`/Engine/EditorBlueprintResources/StandardMacros.IsValid` _returnvalue
          (:`Is Valid`
            (`self.PutIntoBackpack` _returnvalue)
            (return true))
          (:`Is Not Valid`
            (return true))))
      (:`else`
        (return true)))
    (else
      (return true))))

(fn `LookAtCamera`
  (if (`self.LookAt`)
    (bind _characterinbox (`self.CharacterInBox`)
      (:`then`
        (bind _asbp_player_character (cast `/Game/BP/Character/Player/BP_PlayerCharacter` _characterinbox))
        (set `self.L_CameraLocation` (`SceneComponent.K2_GetComponentLocation` (`/Game/BP/Character/Player/BP_PlayerCharacter.Camera` _asbp_player_character)))
        (`SceneComponent.K2_SetWorldRotation` (`self.Text`) (`KismetMathLibrary.FindLookAtRotation` (`SceneComponent.K2_GetComponentLocation` (`self.Text`)) (`self.L_CameraLocation`)) false false))
      (:`else`))))

(fn `PutIntoBackpack`
  (params (InBackpack :type "/Game/BP/Components/BP_BackpackComponent Object Reference")))

(fn `UserConstructionScript`)