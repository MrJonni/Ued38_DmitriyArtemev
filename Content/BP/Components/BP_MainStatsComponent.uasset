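; Actor component that holds an actor's main stats: HP, EP shield, death state and walk speed.
; On BeginPlay it loads its DT_AllStats row by CurrentName, sets character movement for all but one type, then initializes HP/EP.
; The player restores saved values from the GameInstance save unless it is a new game; others start full.
; Damage, heal and shield functions broadcast OnStatsUpdate; damage reduces only HP, ignoring EP.
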(event `self.ReceiveBeginPlay`
  (`self.ConfigureStats`))

(fn `CheckEP`
  (returns (OnMax :type Boolean))
  (return (== (`self.CurrentEP`) (`.MaxEP_13_EA154845465540F625864288521095E8` (break `/Game/BP/Structures/STRUCT_MainStats` (`self.MainStatsStructure`))))))

(fn `CheckHP`
  (returns (OnMax :type Boolean))
  (return (== (`self.CurrentHP`) (`.MaxHP_9_A771449D4D0FB6AC94A77181E18FF634` (break `/Game/BP/Structures/STRUCT_MainStats` (`self.MainStatsStructure`))))))

(fn `ConfigureHealthAndEp`)

(fn `ConfigureMovement`
  (bind ((`MaxWalkSpead_16_033EF0D74DB282E348C12B848A8FEB18` _maxwalkspead)) (break `/Game/BP/Structures/STRUCT_MainStats` (`self.MainStatsStructure`)))
  (if (`|EnumInequality` (`.Type_2_630805404C9DB7C4B38E0DACB86674CA` (break `/Game/BP/Structures/STRUCT_MainStats` (`self.MainStatsStructure`))) "NewEnumerator5")
    (bind _ascharacter (cast `Character` (`self.GetOwner`)))
    (bind _charactermovement (`Character.CharacterMovement` _ascharacter))
    (set `CharacterMovementComponent.MaxWalkSpeed` _maxwalkspead _charactermovement)
    (set `CharacterMovementComponent.MaxWalkSpeedCrouched` (/ _maxwalkspead 2.0) _charactermovement)))

(fn `ConfigureStats`
  (if (!= (`self.CurrentName`) "None")
    (bind _returnvalue (`|GetDataTableRow` "/Game/Data/DT_AllStats.DT_AllStats" (`self.CurrentName`))
      (:`then`
        (set `self.MainStatsStructure` _returnvalue)
        (`|ExecutionSequence`
          (:`then_0`
            (`self.ConfigureMovement`))
          (:`then_1`
            (`self.HPAndEP`))))
      (:`RowNotFound`
        (`KismetSystemLibrary.PrintString` "Configure Stats Failed: Current Name not found in DT" false)))
    (else
      (`KismetSystemLibrary.PrintString` "Configure Stats Failed: Current Name Is Invalid" false))))

(fn `HealUp`
  (params (InToMax :type Boolean :default true) (InAddHP :type Integer))
  (if InToMax
    (set `self.CurrentHP` (`.MaxHP_9_A771449D4D0FB6AC94A77181E18FF634` (break `/Game/BP/Structures/STRUCT_MainStats` (`self.MainStatsStructure`))))
    (else
      (set `self.CurrentHP` (`KismetMathLibrary.Min` (+ (`self.CurrentHP`) (`local.InAddHP`)) (`.MaxHP_9_A771449D4D0FB6AC94A77181E18FF634` (break `/Game/BP/Structures/STRUCT_MainStats` (`self.MainStatsStructure`)))))))
  (`self.OnStatsUpdate` (`self.CurrentHP`) (`self.CurrentEP`) (`self.IsDead`)))

(fn `HPAndEP`
  (bind _savegameobj (`self.NewMacro_0`)
    (:`Is Valid`
      (set `self.CurrentHP` (`/Game/BP/Objects/BP_SaveGame.SavedPlayerHP` _savegameobj))
      (set `self.CurrentEP` (`/Game/BP/Objects/BP_SaveGame.SavedPlayerEP` _savegameobj))
      (`self.OnStatsUpdate` (`self.CurrentHP`) (`self.CurrentEP`) (`self.IsDead`)))
    (:`False`
      (`self.HealUp` true)
      (`self.ShieldUp` true))))

(fn `ReceiveDamage`
  (params (InDamage :type "Float (double-precision)") (InType :type "/Game/BP/Enum/ENUM_DamageType Enum" :default "NewEnumerator0") (InCauser :type "Actor Object Reference"))
  (if (not (`self.IsDead`))
    (set `self.CurrentHP` (- (`self.CurrentHP`) (`KismetMathLibrary.FTrunc` (`local.InDamage`))))
    (if (> (`self.CurrentHP`) 0)
      (set `self.IsDead` false)
      (else
        (set `self.CurrentHP` 0)
        (set `self.IsDead` true)))
    (`self.OnStatsUpdate` (`self.CurrentHP`) (`self.CurrentEP`) (`self.IsDead`) true)))

(fn `ShieldUp`
  (params (InToMax :type Boolean :default true) (InAddEP :type Integer))
  (if InToMax
    (set `self.CurrentEP` (`.MaxEP_13_EA154845465540F625864288521095E8` (break `/Game/BP/Structures/STRUCT_MainStats` (`self.MainStatsStructure`))))
    (else
      (set `self.CurrentEP` (`KismetMathLibrary.Min` (+ (`self.CurrentEP`) (`local.InAddEP`)) (`.MaxEP_13_EA154845465540F625864288521095E8` (break `/Game/BP/Structures/STRUCT_MainStats` (`self.MainStatsStructure`)))))))
  (`self.OnStatsUpdate` (`self.CurrentHP`) (`self.CurrentEP`) (`self.IsDead`)))